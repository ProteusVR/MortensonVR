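; Actor component that draws outlines on its owner by overlaying duplicate meshes with a dynamic line material fed the camera FOV.
; InitializeOutline spawns attached, collision-free copies of all visible skeletal meshes, synced via master pose, plus the one supplied static mesh if visible.
; RefreshOutlines rebuilds the tracked copies, and owner destruction removes them.
; The gated FOV update has no Enter input, since Tick is empty.
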(event Custom|CloseOutline
  (Utilities|FlowControl|Gate true ; enters at Close
    (:Exit
      (if (== (Variables|Default|GetFOVAngle) 0.0)
        (Rendering|Material|SetScalarParameterValue (Variables|Default|GetlineDynamicMaterial) "fov" (Camera|GetFOVAngle (Game|GetPlayerCameraManager 0)) :!class /Script/Engine.MaterialInstanceDynamic)
        (else
          (Rendering|Material|SetScalarParameterValue (Variables|Default|GetlineDynamicMaterial) "fov" (Variables|Default|GetFOVAngle) :!class /Script/Engine.MaterialInstanceDynamic))))))

(event Custom|InitializeOutline
  (params (StaticMeshComponent :type Static%20Mesh%20Component%20Object%20Reference))
  ;[1 1 1] Variable setup: OwnerActor
  (Variables|Default|SetStaticMeshComponent StaticMeshComponent)
  (bind _output_get (Variables|Default|SetOwner%20Actor (Components|GetOwner)))
  ;[1 1 1] Handle Destroying actor
  (Game|BindEventtoOnDestroyed _output_get (delegate Custom|Event%20Destory%20OutlineActors))
  (CallFunction|GererateOutlines))

(event Custom|Event%20Destory%20OutlineActors
  (params (DestroyedActor :type Actor%20Object%20Reference))
  ;[1 1 1] Handle Destroying actor
  (CallFunction|DestroyOutlineActors))

(event Custom|OpenOutline
  (Utilities|FlowControl|Gate true ; enters at Open
    (:Exit
      (if (== (Variables|Default|GetFOVAngle) 0.0)
        (Rendering|Material|SetScalarParameterValue (Variables|Default|GetlineDynamicMaterial) "fov" (Camera|GetFOVAngle (Game|GetPlayerCameraManager 0)) :!class /Script/Engine.MaterialInstanceDynamic)
        (else
          (Rendering|Material|SetScalarParameterValue (Variables|Default|GetlineDynamicMaterial) "fov" (Variables|Default|GetFOVAngle) :!class /Script/Engine.MaterialInstanceDynamic))))))

(event Custom|Event%20Refresh%20Outlines
  ;[1 1 1] To be called when Set Static Mesh / Set Skeletal Mesh is called on the static/skeletal mesh components
  (CallFunction|DestroyOutlineActors)
  (CallFunction|GererateOutlines))

(event EventTick
  (params (DeltaSeconds :type Float%20%28single-precision%29)))

(fn GenSkeletalMeshComponentOutline
  (params (SkeletalMeshComponent :type Skeletal%20Mesh%20Component%20Object%20Reference))
  ;[1 1 1] Variable setup: TargetSkeletalMeshComponent, TargetSkeletalMesh
  (bind _output_get (LocalVariables|SetTargetSkeletalMeshComponent SkeletalMeshComponent))
  (LocalVariables|SetTargetSkeletalMesh (Variables|/Script/Engine.SkinnedMeshComponent|GetSkeletalMesh _output_get))
  ;[1 1 1] Filter only visible mesh components
  (if (Rendering|IsVisible (LocalVariables|GetTargetSkeletalMeshComponent))
    ;[1 1 1] Create a line mesh actor and component by duplicating the owner actor, and transform it the same to the owner actor
    (bind _returnvalue (Game|SpawnActorfromClass "/Game/Proteus_Multi/Outline/SK_APOP.SK_APOP_C" (Transformation|GetActorTransform (Variables|Default|GetOwner%20Actor)) "AlwaysSpawn" 0 0))
    ;[1 1 1] VariableSetup: SkeletalLineMeshActor, SkeletalLineMeshComponent
    (bind _output_get_2 (LocalVariables|SetSkeletalLineMeshActor _returnvalue))
    (LocalVariables|SetSkeletalLineMeshComponent (Variables|/Script/Engine.SkeletalMeshActor|GetSkeletalMeshComponent _output_get_2))
    ;[1 1 1] Add the new actor to the attached actors array
    (Utilities|Array|Add (Variables|Default|GetAttachedOutlineActors) (LocalVariables|GetSkeletalLineMeshActor))
    ;[1 1 1] Attach the line mesh component to the target mesh component
    (Class|SceneComponent|Attachto (LocalVariables|GetSkeletalLineMeshComponent) (LocalVariables|GetTargetSkeletalMeshComponent) "None" "SnapToTargetIncludingScale" false)
    ;[1 1 1] Set the owner actor's skeletal mesh to the line mesh component
    (Class|SkinnedMeshComponent|SetSkeletalMesh (LocalVariables|GetSkeletalLineMeshComponent) (LocalVariables|GetTargetSkeletalMesh) true)
    ;[1 1 1] Disable collision for the line mesh
    (Collision|SetCollisionEnabled (LocalVariables|GetSkeletalLineMeshComponent) "NoCollision")
    ;[1 1 1] Set owner actor's the animation blueprint to the line mesh component.
    (Class|SkinnedMeshComponent|SetMasterPoseComponent (LocalVariables|GetSkeletalLineMeshComponent) (LocalVariables|GetTargetSkeletalMeshComponent) false)
    ;[1 1 1] Set the selected line material to all elements of the line mesh component
    (for (_ _array_index) (Rendering|Material|GetMaterials (LocalVariables|GetSkeletalLineMeshComponent))
      (Rendering|Material|SetMaterial (LocalVariables|GetSkeletalLineMeshComponent) _array_index (Variables|Default|GetlineDynamicMaterial)))
    (return)
    (else
      (return))))

(fn GenStaticMeshComponentOutline
  (params (StaticMeshComponent :type Static%20Mesh%20Component%20Object%20Reference))
  (bind _owner_actor (Variables|Default|GetOwner%20Actor))
  ;[1 1 1] VariableSetup: TargetStaticMeshComponent, TargetStaticMesh
  (bind _output_get (LocalVariables|SetTargetStaticMeshComponent StaticMeshComponent))
  (LocalVariables|SetTargetStaticMesh (Variables|/Script/Engine.StaticMeshComponent|GetStaticMesh _output_get))
  ;[1 1 1] Filter only visible meshes
  (if (Rendering|IsVisible (LocalVariables|GetTargetStaticMeshComponent))
    ;[1 1 1] Create a line mesh actor by duplicating the owner actor, and transform it the same to the owner actor
    (bind _returnvalue (Game|SpawnActorfromClass "/Game/Proteus_Multi/Outline/SM_APOP.SM_APOP_C" (Transformation|GetActorTransform _owner_actor) "AlwaysSpawn" _owner_actor 0))
    ;[1 1 1] VariableSetup: StaticLineMeshActor, StaticLineMeshComponent
    (bind _output_get_2 (LocalVariables|SetStaticLineMeshActor _returnvalue))
    (Utilities|IsValid _output_get_2
      (:Is%20Valid
        (LocalVariables|SetStaticLineMeshComponent (Variables|/Script/Engine.StaticMeshActor|GetStaticMeshComponent _output_get_2))
        ;[1 1 1] Add the new actor to the attached actors array
        (Utilities|Array|Add (Variables|Default|GetAttachedOutlineActors) (LocalVariables|GetStaticLineMeshActor))
        (Transformation|AttachComponentToComponent (LocalVariables|GetStaticLineMeshComponent) (LocalVariables|GetTargetStaticMeshComponent) "None" "SnapToTarget" "SnapToTarget" "SnapToTarget" true)
        (Utilities|IsValid (LocalVariables|GetStaticLineMeshComponent)
          (:Is%20Valid
            (Components|StaticMesh|SetStaticMesh (LocalVariables|GetStaticLineMeshComponent) (LocalVariables|GetTargetStaticMesh))
            ;[1 1 1] Disable collision for the line mesh
            (Collision|SetCollisionEnabled (LocalVariables|GetStaticLineMeshComponent) "NoCollision")
            ;[1 1 1] Set the selected line material to all elements of the line mesh component
            (for (_ _array_index) (Rendering|Material|GetMaterials (LocalVariables|GetStaticLineMeshComponent))
              (Rendering|Material|SetMaterial (LocalVariables|GetStaticLineMeshComponent) _array_index (Variables|Default|GetlineDynamicMaterial)))
            (return)))))
    (else
      (return))))

(fn GererateOutlines
  (bind _returnvalue (Game|GetPlayerCameraManager 0))
  ;[1 1 1] Prepare LineMaterial
  (bind _returnvalue_2 (Rendering|Material|CreateDynamicMaterialInstance (Variables|Default|GetLineMaterial) "None" :!class /Script/Engine.KismetMaterialLibrary))
  (bind _output_get (Variables|Default|SetlineDynamicMaterial _returnvalue_2))
  (Utilities|IsValid _returnvalue
    (:Is%20Valid
      (Rendering|Material|SetScalarParameterValue _output_get "fov" (Camera|GetFOVAngle _returnvalue) :!class /Script/Engine.MaterialInstanceDynamic)
      ;[1 1 1] Generate outlines for all skeletal mesh components
      (for _array_element (Actor|GetComponentsByClass (Variables|Default|GetOwner%20Actor) "/Script/Engine.SkeletalMeshComponent")
        (CallFunction|GenSkeletalMeshComponentOutline _array_element))
      (CallFunction|GenStaticMeshComponentOutline (Variables|Default|GetStaticMeshComponent))
      (return))))

(fn DestroyOutlineActors
  (bind _attachedoutlineactors (Variables|Default|GetAttachedOutlineActors))
  (if (> (Utilities|Array|Length _attachedoutlineactors) 0)
    (for _array_element _attachedoutlineactors
      (Actor|DestroyActor _array_element))
    (Utilities|Array|Clear (Variables|Default|GetAttachedOutlineActors))
    (return)))