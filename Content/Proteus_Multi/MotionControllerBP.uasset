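; Multiplayer VR motion controller for one hand, showing an avatar hand, Oculus Touch or Vive mesh as chosen in VRSettings.
; The authority spawns and attaches the mesh; initialization caches its AnimBP, mirrors left Hands/Touch meshes with negative scale, then opens the Tick gate.
; Tick records the locally controlled HMD transform, via HMDSpace on remotes, and feeds input values to the AnimBP.
; Events handle dash hiding, grab posing and cleanup; an OnRep pushes controller opacity to a material parameter collection.
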(event Custom|DashOnOff
  (params (On :type Boolean))
  ;[1 1 1] Dash
  (Utilities|FlowControl|Sequence
    (:then_0
      (bind _handsmesh (Variables|Settings|GetHandsMesh)
        (:then
          (Rendering|SetActorHiddenInGame _handsmesh On))
        (:else)))
    (:then_1
      (bind _vivecontrollermesh (Variables|Settings|GetViveControllerMesh)
        (:then
          (Rendering|SetActorHiddenInGame _vivecontrollermesh On))
        (:else)))
    (:then_2
      (bind _controllertouch (Variables|Settings|GetControllerTouch)
        (:then
          (Rendering|SetActorHiddenInGame _controllertouch On))
        (:else)))))

(event Custom|AnimGrab
  (params (HandTransform :type Local%20Hand%20Rotations%20STRUCT%20Structure) (Release :type Boolean))
  (bind _animhandavatars (Variables|Animation|GetAnimHandAvatars))
  ;[1 1 0] Update Animations
  (if Release
    (Variables|/Game/Proteus_Multi/HandAssets/OculusAvatar_Hand_AnimBP.OculusAvatar_Hand_AnimBP_C|SetOmega _animhandavatars 0.0)
    (else
      (Variables|/Game/Proteus_Multi/HandAssets/OculusAvatar_Hand_AnimBP.OculusAvatar_Hand_AnimBP_C|SetHandRotations _animhandavatars HandTransform)
      (Variables|/Game/Proteus_Multi/HandAssets/OculusAvatar_Hand_AnimBP.OculusAvatar_Hand_AnimBP_C|SetOmega _animhandavatars 1.0))))

(event Custom|SpawnControllers
  (bind _returnvalue (Transformation|GetActorTransform))
  (bind _self self)
  (bind _vrsettings (Variables|Settings|GetVRSettings))
  (bind (_controllermesh _controlleropacity) (Utilities|Struct|BreakVRSettings _vrsettings))
  ;[0.3086 1 0.318] Spawn Controller
  (switch Utilities|FlowControl|Switch|SwitchonControllerEnum _controllermesh
    (:NewEnumerator0
      (bind _returnvalue_2 (Game|SpawnActorfromClass "/Game/Proteus_Multi/HandAssets/CVR_Hand_BP.CVR_Hand_BP_C" _returnvalue "AlwaysSpawn" _self 0))
      (bind _output_get (Variables|Settings|SetHandsMesh _returnvalue_2))
      (Transformation|AttachComponentToComponent _output_get (Variables|Default|GetMCRoot) "None" "SnapToTarget" "SnapToTarget" "SnapToTarget" true))
    (:NewEnumerator1
      (bind _returnvalue_3 (Game|SpawnActorfromClass "/Game/Proteus_Multi/TouchControllers/Controller_Touch_BP_C.Controller_Touch_BP_C_C" _returnvalue "AlwaysSpawn" _self 0))
      (bind _output_get_2 (Variables|Settings|SetControllerTouch _returnvalue_3))
      (Transformation|AttachComponentToComponent _output_get_2 (Variables|Default|GetMCRoot) "None" "SnapToTarget" "SnapToTarget" "SnapToTarget" true))
    (:NewEnumerator2
      (bind _returnvalue_4 (Game|SpawnActorfromClass "/Game/Proteus_Multi/ViveControllers/ViveController_BP.ViveController_BP_C" _returnvalue "AlwaysSpawn" _self 0))
      (bind _output_get_3 (Variables|Settings|SetViveControllerMesh _returnvalue_4))
      (Transformation|AttachComponentToComponent _output_get_3 (Variables|Default|GetMCRoot) "None" "SnapToTarget" "SnapToTarget" "SnapToTarget" true)))
  (Variables|Settings|SetController%20Opacity _controlleropacity)
  (CallFunction|ControllerInitialization))

(event Custom|UpdateAnim
  (bind _animbp_touch (Variables|Animation|GetAnimBP_Touch))
  (bind _animhandavatars (Variables|Animation|GetAnimHandAvatars))
  ;[1 1 0] Update Animations
  (switch Utilities|FlowControl|Switch|SwitchonControllerEnum (.ControllerMesh (Utilities|Struct|BreakVRSettings (Variables|Settings|GetVRSettings)))
    (:NewEnumerator0
      (Variables|/Game/Proteus_Multi/HandAssets/OculusAvatar_Hand_AnimBP.OculusAvatar_Hand_AnimBP_C|SetThumbPosition _animhandavatars (Variables|Animation|GetThumbPosition))
      (Variables|/Game/Proteus_Multi/HandAssets/OculusAvatar_Hand_AnimBP.OculusAvatar_Hand_AnimBP_C|SetIndexPosition _animhandavatars (Variables|Animation|GetIndexPosition))
      (Variables|/Game/Proteus_Multi/HandAssets/OculusAvatar_Hand_AnimBP.OculusAvatar_Hand_AnimBP_C|SetHandPosition _animhandavatars (Variables|Animation|GetHandPosition)))
    (:NewEnumerator1
      (Variables|/Game/Proteus_Multi/TouchControllers/Controller_Touch_AnimBlueprintC.Controller_Touch_AnimBlueprintC_C|SetLower_Pressure _animbp_touch (Variables|Animation|GetTLowerPosition))
      (Variables|/Game/Proteus_Multi/TouchControllers/Controller_Touch_AnimBlueprintC.Controller_Touch_AnimBlueprintC_C|SetUpper_Pressure _animbp_touch (Variables|Animation|GetTUpperPosition))
      (Variables|/Game/Proteus_Multi/TouchControllers/Controller_Touch_AnimBlueprintC.Controller_Touch_AnimBlueprintC_C|SetHand_Pressure _animbp_touch (Variables|Animation|GetTHandPosition))
      (Variables|/Game/Proteus_Multi/TouchControllers/Controller_Touch_AnimBlueprintC.Controller_Touch_AnimBlueprintC_C|SetIndex_Pressure _animbp_touch (Variables|Animation|GetTIndexPosition))
      (Variables|/Game/Proteus_Multi/TouchControllers/Controller_Touch_AnimBlueprintC.Controller_Touch_AnimBlueprintC_C|SetThumbStick_Rotation _animbp_touch (Variables|Animation|GetTThumbStickRotation)))
    (:NewEnumerator2
      (Variables|/Game/Proteus_Multi/ViveControllers/Vive_Controller_V2_Skeleton_AnimBlueprint.Vive_Controller_V2_Skeleton_AnimBlueprint_C|SetTriggerAxisAmount (Variables|Animation|GetAnimBP_Vive) (Variables|Animation|GetTriggerAxis)))))

(event Custom|StartComponent
  ;[0.9663 0.3338 1] Initial Settings
  (Utilities|FlowControl|Delay 0.2)
  (switch Utilities|FlowControl|Switch|SwitchonHandEnum (Variables|Settings|GetHandSide)
    (:NewEnumerator0
      _)
    (:NewEnumerator1
      _))
  (Networking|SwitchHasAuthority
    (:Authority
      (CallFunction|SpawnControllers))
    (:Remote
      (CallFunction|ControllerInitialization))))

(event Custom|Open%20Tick
  (bind (_devicerotation _deviceposition) (Class|HeadMountedDisplayFunctionLibrary|GetOrientationandPosition))
  (bind _returnvalue (Components|GetOwner))
  (bind _returnvalue_2 (Math|Transform|MakeTransform _deviceposition _devicerotation))
  (bind _instigator (Variables|/Script/Engine.Actor|GetInstigator _returnvalue))
  (bind _returnvalue_3 (Pawn|IsLocallyControlled _instigator))
  ;[0.5665 0.7455 1] Main Tick
  (Utilities|FlowControl|Gate true) ; enters at Open
)

(event Custom|Controller%20Initialization
  (bind _vivecontrollermesh (Variables|Settings|GetViveControllerMesh))
  (bind _handsmesh (Variables|Settings|GetHandsMesh))
  (bind _vrsettings (Variables|Settings|GetVRSettings))
  (bind (_controllermesh _vivecontrollerskin _avatarcolor_singleplayeronly) (Utilities|Struct|BreakVRSettings _vrsettings))
  ;[0.4855 1 0.8167] Controller Initialization
  (CallFunction|SetControllersTransforms)
  (switch Utilities|FlowControl|Switch|SwitchonControllerEnum _controllermesh
    (:NewEnumerator0
      (Default|DynamicMaterial _handsmesh _avatarcolor_singleplayeronly)
      (bind _asoculus_avatar_hand_anim_bp (Utilities|Casting|CastToOculusAvatar_Hand_AnimBP (Components|SkeletalMesh|GetAnimInstance (Variables|/Game/Proteus_Multi/HandAssets/CVR_Hand_BP.CVR_Hand_BP_C|GetVR_HandSM _handsmesh))))
      (Variables|Animation|SetAnimHandAvatars _asoculus_avatar_hand_anim_bp))
    (:NewEnumerator1
      (bind _ascontroller_touch_anim_blueprint_c (Utilities|Casting|CastToController_Touch_AnimBlueprintC (Components|SkeletalMesh|GetAnimInstance (Variables|/Game/Proteus_Multi/TouchControllers/Controller_Touch_BP_C.Controller_Touch_BP_C_C|GetTouchSM (Variables|Settings|GetControllerTouch)))))
      (Variables|Animation|SetAnimBP_Touch _ascontroller_touch_anim_blueprint_c))
    (:NewEnumerator2
      (Default|SetMaterial _vivecontrollermesh (Utilities|Array|Get(acopy) (Variables|Settings|GetViveMaterial) (Math|Conversions|ToInteger(Byte) _vivecontrollerskin)))
      (bind _asvive_controller_v2_skeleton_anim_blueprint (Utilities|Casting|CastToVive_Controller_V2_Skeleton_AnimBlueprint (Components|SkeletalMesh|GetAnimInstance (Variables|/Game/Proteus_Multi/ViveControllers/ViveController_BP.ViveController_BP_C|GetVive_Controller _vivecontrollermesh))))
      (Variables|Animation|SetAnimBP_Vive _asvive_controller_v2_skeleton_anim_blueprint)))
  (CallFunction|OpenTick))

(event Custom|HMD%20Space
  (params (HMDTransform :type Transform))
  ;[0.5665 0.7455 1] Main Tick
  (Variables|Teleportation|SetHMDRelativePosition HMDTransform))

(event EventDestroyed
  ;[1 1 1] Event Destroyed
  (Utilities|FlowControl|Sequence
    (:then_0
      (bind _handsmesh (Variables|Settings|GetHandsMesh)
        (:then
          (Actor|DestroyActor _handsmesh))
        (:else)))
    (:then_1
      (bind _vivecontrollermesh (Variables|Settings|GetViveControllerMesh)
        (:then
          (Actor|DestroyActor _vivecontrollermesh))
        (:else)))
    (:then_2
      (bind _controllertouch (Variables|Settings|GetControllerTouch)
        (:then
          (Actor|DestroyActor _controllertouch))
        (:else)))))

(event EventTick
  (params (DeltaSeconds :type Float%20%28single-precision%29))
  (bind (_devicerotation _deviceposition) (Class|HeadMountedDisplayFunctionLibrary|GetOrientationandPosition))
  (bind _returnvalue (Components|GetOwner))
  (bind _returnvalue_2 (Math|Transform|MakeTransform _deviceposition _devicerotation))
  (bind _instigator (Variables|/Script/Engine.Actor|GetInstigator _returnvalue))
  (bind _returnvalue_3 (Pawn|IsLocallyControlled _instigator))
  ;[0.5665 0.7455 1] Main Tick
  (Utilities|FlowControl|Gate true
    (:Exit
      (Utilities|FlowControl|Sequence
        (:then_0
          (Networking|SwitchHasAuthority
            (:Authority
              (if _returnvalue_3
                (Variables|Teleportation|SetHMDRelativePosition _returnvalue_2)))))
        (:then_1
          (Networking|SwitchHasAuthority
            (:Remote
              (if _returnvalue_3
                (CallFunction|HMDSpace _returnvalue_2)))))
        (:then_2
          (CallFunction|UpdateAnim))))))

(fn ConstructionScript)

(fn OnRepControllerOpacity
  (Rendering|Material|SetScalarParameterValue "/Game/Proteus_Multi/Materials/Opacity_C.Opacity_C" "Opacity_Controls" (Variables|Settings|GetController%20Opacity) :!class /Script/Engine.KismetMaterialLibrary))

(fn SetControllersTransforms
  (switch Utilities|FlowControl|Switch|SwitchonControllerEnum (.ControllerMesh (Utilities|Struct|BreakVRSettings (Variables|Settings|GetVRSettings)))
    (:NewEnumerator0
      (switch Utilities|FlowControl|Switch|SwitchonHandEnum (Variables|Settings|GetHandSide)
        (:NewEnumerator0
          (Transformation|SetRelativeTransform (Variables|/Game/Proteus_Multi/HandAssets/CVR_Hand_BP.CVR_Hand_BP_C|GetVR_HandSM (Variables|Settings|GetHandsMesh)) (Math|Transform|MakeTransform "-3.800000,0.700000,0.000000" "90.000000,0.000000,90.000000" "1.000000,1.000000,-1.000000") false false))))
    (:NewEnumerator1
      (switch Utilities|FlowControl|Switch|SwitchonHandEnum (Variables|Settings|GetHandSide)
        (:NewEnumerator0
          (Transformation|SetRelativeTransform (Variables|/Game/Proteus_Multi/TouchControllers/Controller_Touch_BP_C.Controller_Touch_BP_C_C|GetTouchSM (Variables|Settings|GetControllerTouch)) (Math|Transform|MakeTransform "0, 0, 0" "0.000000,180.000000,0.000000" "1.000000,1.000000,-1.000000") false false))))))