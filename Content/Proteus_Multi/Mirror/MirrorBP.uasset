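; Mirror actor that shows a scene capture on a plane through a render target.
; The construction script adds a non-colliding instanced plane with Mirror_MAT, then attaches a new SceneCaptureComponent2D to it that writes to MirrorRenderTarget.
; BeginPlay only runs a one-second delay.
; The VR headset switches in both graphs are disconnected, including a smaller-scale copy of the mirror setup in the event graph.
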(event EventBeginPlay
  (Utilities|FlowControl|Delay 1.0))

(fn ConstructionScript
  (bind _instancedstaticmesh (Variables|Default|GetInstancedStaticMesh))
  (Components|InstancedStaticMesh|AddInstance _instancedstaticmesh (Math|Transform|MakeTransform "0, 0, 0" "0.000000,0.000000,-90.000000" "2.000000,2.000000,2.000000"))
  (Components|StaticMesh|SetStaticMesh _instancedstaticmesh "/Game/Proteus_Multi/Mirror/Plane1.Plane1")
  (Collision|SetCollisionEnabled _instancedstaticmesh "NoCollision")
  (Rendering|Material|SetMaterial _instancedstaticmesh 0 "/Game/Proteus_Multi/Mirror/Mirror_MAT.Mirror_MAT")
  (bind _returnvalue (AddComponent|AddSceneCaptureComponent2D false (Math|Transform|MakeTransform "0, 0, 0" "90.000000,0.000000,0.000000")))
  (Variables|/Script/Engine.SceneCaptureComponent2D|SetTextureTarget _returnvalue "/Game/Proteus_Multi/Mirror/MirrorRenderTarget.MirrorRenderTarget")
  (Transformation|AttachComponentToComponent _returnvalue (Variables|Default|GetInstancedStaticMesh) "None" "SnapToTarget" "SnapToTarget" "SnapToTarget" true)
  (Transformation|SetRelativeTransform _returnvalue (Math|Transform|MakeTransform "0, 0, 0" "0.000000,-90.000000,180.000000" "0.500000,0.500000,0.500000") false false))