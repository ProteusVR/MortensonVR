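; Fire alarm Blueprint for the Mortenson level that places a fixed set of fire alarm meshes as a single actor.
; The Construction Script adds six unrotated, unit-scale instances to a Hierarchical Instanced Static Mesh at hardcoded local offsets, batching their rendering.
; The event graph holds only empty default events, so the actor has no runtime or alarm behavior.
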(event EventBeginPlay)

(event Collision|EventActorBeginOverlap
  (params (OtherActor :type Actor%20Object%20Reference)))

(event EventTick
  (params (DeltaSeconds :type Float%20%28single-precision%29)))

(fn ConstructionScript
  (Components|InstancedStaticMesh|AddInstance (Variables|Default|GetHierarchicalInstancedStaticMesh) (Math|Transform|MakeTransform "0, 0, 0"))
  (Components|InstancedStaticMesh|AddInstance (Variables|Default|GetHierarchicalInstancedStaticMesh) (Math|Transform|MakeTransform "766.000000,1844.000000,-4.000000"))
  (Components|InstancedStaticMesh|AddInstance (Variables|Default|GetHierarchicalInstancedStaticMesh) (Math|Transform|MakeTransform "1340.000000,1753.000000,0.000000" "0, 0,0.000000"))
  (Components|InstancedStaticMesh|AddInstance (Variables|Default|GetHierarchicalInstancedStaticMesh) (Math|Transform|MakeTransform "613.000000,1020.000000,-43.000000"))
  (Components|InstancedStaticMesh|AddInstance (Variables|Default|GetHierarchicalInstancedStaticMesh) (Math|Transform|MakeTransform "900.000000,486.000000,0.000000" "0, 0,0.000000"))
  (Components|InstancedStaticMesh|AddInstance (Variables|Default|GetHierarchicalInstancedStaticMesh) (Math|Transform|MakeTransform "3.000000,1730.000000,0.000000")))