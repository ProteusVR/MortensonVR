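; Wire_BP is an actor that lays out a fixed arrangement of mesh instances, likely wire props going by its name.
; Its construction script adds six unrotated, unit-scale instances to a Hierarchical Instanced Static Mesh component in two rows of three at hard-coded, unevenly spaced offsets.
; The event graph holds only disabled placeholder events, so it has no runtime logic.
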(event EventBeginPlay)

(event Collision|EventActorBeginOverlap
  (params (OtherActor :type Actor%20Object%20Reference)))

(event EventTick
  (params (DeltaSeconds :type Float%20%28single-precision%29)))

(fn ConstructionScript
  (Components|InstancedStaticMesh|AddInstance (Variables|Default|GetHierarchicalInstancedStaticMesh) (Math|Transform|MakeTransform "0, 0, 0"))
  (Components|InstancedStaticMesh|AddInstance (Variables|Default|GetHierarchicalInstancedStaticMesh) (Math|Transform|MakeTransform "259.000000,2.000000,0.000000"))
  (Components|InstancedStaticMesh|AddInstance (Variables|Default|GetHierarchicalInstancedStaticMesh) (Math|Transform|MakeTransform "624.000000,2.000000,0.000000"))
  (Components|InstancedStaticMesh|AddInstance (Variables|Default|GetHierarchicalInstancedStaticMesh) (Math|Transform|MakeTransform "0.000000,-272.000000,0.000000"))
  (Components|InstancedStaticMesh|AddInstance (Variables|Default|GetHierarchicalInstancedStaticMesh) (Math|Transform|MakeTransform "259.000000,-272.000000,0.000000"))
  (Components|InstancedStaticMesh|AddInstance (Variables|Default|GetHierarchicalInstancedStaticMesh) (Math|Transform|MakeTransform "624.000000,-272.000000,0.000000")))